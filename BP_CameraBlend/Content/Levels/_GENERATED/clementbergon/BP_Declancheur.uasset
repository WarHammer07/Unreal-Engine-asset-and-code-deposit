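; BP_Declancheur is a one-shot trigger volume that drops a block and shifts the player's view to another camera.
; On BeginPlay it caches the first-person character.
; Any overlap with its Box enables physics on BPBloc's mesh, starts a five-second eased blend to CameraActive, and destroys the trigger.
; Player input is disabled and re-enabled within the same sequence, without waiting for the blend.
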(event `self.ReceiveBeginPlay`
  (bind _asbp_first_person_character (cast `/Game/FirstPerson/Blueprints/BP_FirstPersonCharacter` (`GameplayStatics.GetPlayerCharacter` 0)))
  (set `self.Joueur` _asbp_first_person_character))

(event `self.Box.OnComponentBeginOverlap`
  (params (OverlappedComponent :type "PrimitiveComponent Object Reference") (OtherActor :type "Actor Object Reference") (OtherComp :type "PrimitiveComponent Object Reference") (OtherBodyIndex :type Integer) (bFromSweep :type Boolean) (SweepResult :type "HitResult Structure (by ref)"))
  (bind _bp_bloc (`self.BP_Bloc`))
  (`|ExecutionSequence`
    (:`then_0`
      (`/Engine/EditorBlueprintResources/StandardMacros.IsValid` _bp_bloc
        (:`Is Valid`
          (`PrimitiveComponent.SetSimulatePhysics` (`/Game/Levels/_GENERATED/clementbergon/BP_Bloc.SM_Bloc` _bp_bloc) true))))
    (:`then_1`
      (`self.DisableInput` (`self.Joueur`) null))
    (:`then_2`
      (`PlayerController.SetViewTargetWithBlend` (`GameplayStatics.GetPlayerController` 0) (`self.CameraActive`) 5.0 "VTBlend_EaseInOut" 1.0 false))
    (:`then_3`
      (`self.EnableInput` (`self.Joueur`) null)
      (`self.K2_DestroyActor`))))

(fn `UserConstructionScript`)