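; BP_SpawnerBig is a spawner that releases a set number of BP_Monster AI pawns.
; On BeginPlay it copies NumBigMonster into a countdown and waits a short initial delay.
; A delay-driven loop then spawns one monster at a time, randomly at one of the first two SpawnPoint entries, with VitesseSpawn as the interval, until the countdown runs out.
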(event `self.ReceiveBeginPlay`
  (set `self.NbrBigMonster` (`self.NumBigMonster`))
  (`KismetSystemLibrary.Delay` 5.0)
  (if (> (`self.NbrBigMonster`) 0) :!label _label
    (`AIBlueprintHelperLibrary.SpawnAIFromClass` "/Game/ThirdPerson/Blueprints/BP_Monster.BP_Monster_C" null (`SceneComponent.K2_GetComponentLocation` (`/Game/Personnages/Spawner/BP_SpawPointBig.SpawnPoint` (`|GetArrayItem` (`self.SpawnPoint`) (`KismetMathLibrary.RandomIntegerInRange` 0 1)))) (struct) false null)
    (`/Engine/EditorBlueprintResources/StandardMacros.DecrementInt` (`self.NbrBigMonster`)
      (:`  `
        (`KismetSystemLibrary.Delay` (`KismetMathLibrary.Conv_IntToDouble` (`self.VitesseSpawn`)))
        (goto _label)))))

(fn `UserConstructionScript`)