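; BP_SpawnerSmall is a spawner that releases a set number of BP_Ennemis AI enemies, counted as small monsters.
; On BeginPlay it copies NumSmallMonster into a countdown and waits briefly before the first spawn.
; A delayed loop then spawns one enemy per pass at a random pick of the first two SpawnPoints, paced by VitesseSpawn, until the count reaches zero.
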(event `self.ReceiveBeginPlay`
  (set `self.NbrSmallMonster` (`self.NumSmallMonster`))
  (`KismetSystemLibrary.Delay` 5.0)
  (if (> (`self.NbrSmallMonster`) 0) :!label _label
    (`AIBlueprintHelperLibrary.SpawnAIFromClass` "/Game/ThirdPerson/Blueprints/BP_Ennemis.BP_Ennemis_C" null (`SceneComponent.K2_GetComponentLocation` (`/Game/Personnages/Spawner/BP_SpawPointSmall.SpawnPoint` (`|GetArrayItem` (`self.SpawnPoints`) (`KismetMathLibrary.RandomIntegerInRange` 0 1)))) (struct) false null)
    (`/Engine/EditorBlueprintResources/StandardMacros.DecrementInt` (`self.NbrSmallMonster`)
      (:`  `
        (`KismetSystemLibrary.Delay` (`KismetMathLibrary.Conv_IntToDouble` (`self.VitesseSpawn`)))
        (goto _label)))))

(fn `UserConstructionScript`)