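; BP_Porte_02 is a double sliding door that opens when the player enters its Zone volume and closes when they leave.
; The construction script stores each panel's relative start position, derives open positions by offsetting Y in opposite directions by Ouverture, and sets the timeline play rate from Vitesse.
; Overlap events play or reverse the timeline, whose AnimPorte curve lerps both panels between those positions.
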(event `self.Zone.OnComponentBeginOverlap`
  (params (OverlappedComponent :type "PrimitiveComponent Object Reference") (OtherActor :type "Actor Object Reference") (OtherComp :type "PrimitiveComponent Object Reference") (OtherBodyIndex :type Integer) (bFromSweep :type Boolean) (SweepResult :type "HitResult Structure (by ref)"))
  ; On test si c'est bien le joueur qui entre dans le volume
  (if (== OtherActor (`GameplayStatics.GetPlayerCharacter` 0))
    (bind (_direction _animporte) (`Timeline|Timeline` :!label _label)
      (:`Update`
        ; Déplacement porte GAUCHE
        (`SceneComponent.K2_SetRelativeLocation` (`self.Porte_G`) (`KismetMathLibrary.VLerp` (`self.PosDepG`) (`self.PosArrG`) _animporte) false false)
        ; Déplacement porte DROITE
        (`SceneComponent.K2_SetRelativeLocation` (`self.Porte_D`) (`KismetMathLibrary.VLerp` (`self.PosDepD`) (`self.PosArrD`) _animporte) false false)))))

(event `self.Zone.OnComponentEndOverlap`
  (params (OverlappedComponent :type "PrimitiveComponent Object Reference") (OtherActor :type "Actor Object Reference") (OtherComp :type "PrimitiveComponent Object Reference") (OtherBodyIndex :type Integer))
  ; On test si c'est bien le joueur qui sort dans le volume
  (if (== OtherActor (`GameplayStatics.GetPlayerCharacter` 0))
    (goto _label :!via `Reverse`)))

(fn `UserConstructionScript`
  (bind _ouverture (`self.Ouverture`))
  (`|ExecutionSequence`
    (:`then_0`
      ; Enregistrement de la position des 2 portes (vont être utilisées pour plus tard)
      (bind _output_get (set `self.PosDepG` (`SceneComponent.RelativeLocation` (`self.Porte_G`))))
      ; Enregistrement de la position des portes à l'arrivée
      (set `self.PosArrG` (`KismetMathLibrary.MakeVector` (.x _output_get) (- (.y _output_get) _ouverture) (.z _output_get))))
    (:`then_1`
      (bind _output_get_2 (set `self.PosDepD` (`SceneComponent.RelativeLocation` (`self.Porte_D`))))
      (set `self.PosArrD` (`KismetMathLibrary.MakeVector` (.x _output_get_2) (+ (.y _output_get_2) _ouverture) (.z _output_get_2))))
    (:`then_2`
      ; Définition du play rate (vitesse de lecture)
      (`TimelineComponent.SetPlayRate` (`self.Timeline`) (`self.Vitesse`)))))