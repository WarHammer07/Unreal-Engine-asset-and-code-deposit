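; BP_DéclencheurLapin is a trigger volume that opens doors while a rabbit actor (BP_Lapin) is inside it.
; Begin and end overlaps on ZoneDeCollision cast the other actor to BP_Lapin, then call Ouvre or Ferme on every entry in Portes.
; The construction script fills Portes with all BP_Porte_03 actors in the level, so each trigger drives every such door.
; Player-character checks remain in the graph but never run.
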(event `self.Zone de collision.OnComponentBeginOverlap`
  (params (OverlappedComponent :type "PrimitiveComponent Object Reference") (OtherActor :type "Actor Object Reference") (OtherComp :type "PrimitiveComponent Object Reference") (OtherBodyIndex :type Integer) (bFromSweep :type Boolean) (SweepResult :type "HitResult Structure (by ref)"))
  ; On compare l'objet qui vient de rentrer avec BP_Lapin
  (cast `/Game/Acteurs/Mur/BP_Lapin` OtherActor)
  (for _array_element (`self.Portes`)
    (`/Game/Acteurs/Mur/BP_Porte_03.Ouvre` _array_element)))

(event `self.Zone de collision.OnComponentEndOverlap`
  (params (OverlappedComponent :type "PrimitiveComponent Object Reference") (OtherActor :type "Actor Object Reference") (OtherComp :type "PrimitiveComponent Object Reference") (OtherBodyIndex :type Integer))
  ; On compare l'objet qui vient de rentrer avec BP_Lapin
  (cast `/Game/Acteurs/Mur/BP_Lapin` OtherActor)
  (for _array_element (`self.Portes`)
    (`/Game/Acteurs/Mur/BP_Porte_03.Ferme` _array_element)))

(fn `UserConstructionScript`
  (bind _outactors (`GameplayStatics.GetAllActorsOfClass` "/Game/Acteurs/Mur/BP_Porte_03.BP_Porte_03_C"))
  (set `self.Portes` _outactors))