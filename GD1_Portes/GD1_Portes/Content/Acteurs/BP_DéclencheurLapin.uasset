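; BP_DéclencheurLapin is a trigger zone that opens doors while the rabbit BP_Lapinou stands in it.
; The construction script fills Portes with every BP_Porte_03 actor in the level, so the trigger drives all of them.
; Begin and end overlaps on Zone cast the other actor to BP_Lapinou, then call Ouvre or Ferme on each door.
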(event `self.Zone.OnComponentBeginOverlap`
  (params (OverlappedComponent :type "PrimitiveComponent Object Reference") (OtherActor :type "Actor Object Reference") (OtherComp :type "PrimitiveComponent Object Reference") (OtherBodyIndex :type Integer) (bFromSweep :type Boolean) (SweepResult :type "HitResult Structure (by ref)"))
  ; On compare l'objet qui vient de rentrer avec BP_Lapinou
  (cast `/Game/Acteurs/BP_Lapinou` OtherActor)
  ; On demande à la porte d'éxécuter la bonne action
  (for _array_element (`self.Portes`)
    (`/Game/Acteurs/BP_Porte_03.Ouvre` _array_element)))

(event `self.Zone.OnComponentEndOverlap`
  (params (OverlappedComponent :type "PrimitiveComponent Object Reference") (OtherActor :type "Actor Object Reference") (OtherComp :type "PrimitiveComponent Object Reference") (OtherBodyIndex :type Integer))
  ; On compare l'objet qui vient de rentrer avec BP_Lapinou
  (cast `/Game/Acteurs/BP_Lapinou` OtherActor)
  ; On demande à la porte d'éxécuter la bonne action
  (for _array_element (`self.Portes`)
    (`/Game/Acteurs/BP_Porte_03.Ferme` _array_element)))

(fn `UserConstructionScript`
  (bind _outactors (`GameplayStatics.GetAllActorsOfClass` "/Game/Acteurs/BP_Porte_03.BP_Porte_03_C"))
  (set `self.Portes` _outactors))