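; BP_Déclencheur is a trigger volume that opens and closes doors as the player enters and leaves it.
; Its construction script fills the Portes array with every BP_Porte_03 actor in the level, so one trigger drives all doors of that class.
; The Zone overlap events react only to player character 0, calling Ouvre on each door on entry and Ferme on exit.
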(event `self.Zone.OnComponentBeginOverlap`
  (params (OverlappedComponent :type "PrimitiveComponent Object Reference") (OtherActor :type "Actor Object Reference") (OtherComp :type "PrimitiveComponent Object Reference") (OtherBodyIndex :type Integer) (bFromSweep :type Boolean) (SweepResult :type "HitResult Structure (by ref)"))
  ; On test si c'est bien le joueur qui entre dans le volume
  (if (== OtherActor (`GameplayStatics.GetPlayerCharacter` 0))
    (for _array_element (`self.Portes`)
      (`/Game/Acteurs/BP_Porte_03.Ouvre` _array_element))))

(event `self.Zone.OnComponentEndOverlap`
  (params (OverlappedComponent :type "PrimitiveComponent Object Reference") (OtherActor :type "Actor Object Reference") (OtherComp :type "PrimitiveComponent Object Reference") (OtherBodyIndex :type Integer))
  ; On test si c'est bien le joueur qui sort dans le volume
  (if (== OtherActor (`GameplayStatics.GetPlayerCharacter` 0))
    (for _array_element (`self.Portes`)
      (`/Game/Acteurs/BP_Porte_03.Ferme` _array_element))))

(fn `UserConstructionScript`
  (bind _outactors (`GameplayStatics.GetAllActorsOfClass` "/Game/Acteurs/BP_Porte_03.BP_Porte_03_C"))
  (set `self.Portes` _outactors))