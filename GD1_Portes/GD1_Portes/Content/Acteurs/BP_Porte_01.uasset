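; BP_Porte_01 is an automatic double sliding door that opens while the player character is inside its Zone volume.
; The construction script records the starting relative location of both panels, PorteG and PorteD.
; On begin overlap, MoveComponentTo eases the panels apart in opposite directions along local Y; on end overlap it returns them, much faster.
; Both transitions play the Audio component's sound from the start.
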(event `self.Zone.OnComponentBeginOverlap`
  (params (OverlappedComponent :type "PrimitiveComponent Object Reference") (OtherActor :type "Actor Object Reference") (OtherComp :type "PrimitiveComponent Object Reference") (OtherBodyIndex :type Integer) (bFromSweep :type Boolean) (SweepResult :type "HitResult Structure (by ref)"))
  ; On test si c'est bien le joueur qui entre dans le volume
  (if (== OtherActor (`GameplayStatics.GetPlayerCharacter` 0))
    (`|ExecutionSequence`
      (:`then_0`
        (`KismetSystemLibrary.MoveComponentTo` (`self.Porte_G`) (- (`self.PosDepG`) (0.0 110.0 0.0)) (struct) true true 1.0))
      (:`then_1`
        (`KismetSystemLibrary.MoveComponentTo` (`self.Porte_D`) (+ (`self.PosDepD`) (0.0 110.0 0.0)) (struct) true true 1.0))
      (:`then_2`
        (`AudioComponent.Play` (`self.Audio`) 0.0)))))

(event `self.Zone.OnComponentEndOverlap`
  (params (OverlappedComponent :type "PrimitiveComponent Object Reference") (OtherActor :type "Actor Object Reference") (OtherComp :type "PrimitiveComponent Object Reference") (OtherBodyIndex :type Integer))
  ; On test si c'est bien le joueur qui sort dans le volume
  (if (== OtherActor (`GameplayStatics.GetPlayerCharacter` 0))
    (`|ExecutionSequence`
      (:`then_0`
        (`KismetSystemLibrary.MoveComponentTo` (`self.Porte_G`) (`self.PosDepG`) (struct) true true 0.2))
      (:`then_1`
        (`KismetSystemLibrary.MoveComponentTo` (`self.Porte_D`) (`self.PosDepD`) (struct) true true 0.2))
      (:`then_2`
        (`AudioComponent.Play` (`self.Audio`) 0.0)))))

(fn `UserConstructionScript`
  (`|ExecutionSequence`
    (:`then_0`
      ; Enregistrement de la position des 2 portes (vont être utilisées plus tard)
      (set `self.PosDepG` (`SceneComponent.RelativeLocation` (`self.Porte_G`))))
    (:`then_1`
      (set `self.PosDepD` (`SceneComponent.RelativeLocation` (`self.Porte_D`))))))