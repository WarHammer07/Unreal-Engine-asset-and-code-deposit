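; BP_Dalles is a numbered floor tile that enters its digit into a door code when stepped on.
; The construction script displays Chiffre on the tile and caches the BP_DoorFrame found in the level.
; An overlap while inactive lowers the slab, plays audio, turns the number green and passes Chiffre to the door's MAJCode.
; After a two-second delay the slab rises, re-arms and resets the number color.
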(event `self.Box.OnComponentBeginOverlap`
  (params (OverlappedComponent :type "PrimitiveComponent Object Reference") (OtherActor :type "Actor Object Reference") (OtherComp :type "PrimitiveComponent Object Reference") (OtherBodyIndex :type Integer) (bFromSweep :type Boolean) (SweepResult :type "HitResult Structure (by ref)"))
  (if (not (`self.IsActive`))
    (`|ExecutionSequence`
      (:`then_0`
        (`SceneComponent.K2_AddLocalOffset` (`self.SM_Dalle`) (0.0 0.0 -5.0) false false)
        (set `self.IsActive` true)
        (`KismetSystemLibrary.Delay` 2.0)
        (`|ExecutionSequence`
          (:`then_0`
            (`SceneComponent.K2_AddLocalOffset` (`self.SM_Dalle`) (0.0 0.0 5.0) false false)
            (set `self.IsActive` false))
          (:`then_1`
            (`TextRenderComponent.SetTextRenderColor` (`self.Number`) (make `Color` 1 1 1 1)))))
      (:`then_1`
        (`AudioComponent.Play` (`self.Audio`) 0.0))
      (:`then_2`
        (`TextRenderComponent.SetTextRenderColor` (`self.Number`) (make `Color` 0 100)))
      (:`then_3`
        (`/Game/LevelPrototyping/Interactable/Door/BP_DoorFrame.MAJCode` (`self.Door`) (`self.chiffre`))))))

(fn `UserConstructionScript`
  (`|ExecutionSequence`
    (:`then_0`
      (`TextRenderComponent.K2_SetText` (`self.Number`) (`KismetTextLibrary.Conv_IntToText` (`self.chiffre`))))
    (:`then_1`
      (bind _returnvalue (`GameplayStatics.GetActorOfClass` "/Game/LevelPrototyping/Interactable/Door/BP_DoorFrame.BP_DoorFrame_C"))
      (set `self.Door` _returnvalue))))