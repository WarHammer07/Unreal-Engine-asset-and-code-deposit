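; Light actor that gives visual feedback on a password attempt through its point light.
; GoodPassword turns the light bright green for a timed period, and BadPassword turns it bright red for a shorter one.
; Each event uses a delay, then switches the light off by setting its intensity to zero.
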(event `GoodPassword`
  (`LightComponent.SetLightColor` (`self.PointLight`) (make `LinearColor` 0.0 1.0 0.0 1.0) true)
  (`LightComponent.SetIntensity` (`self.PointLight`) 10000.0)
  (`KismetSystemLibrary.Delay` 10.0)
  (`LightComponent.SetIntensity` (`self.PointLight`) 0.0))

(event `BadPassword`
  (`LightComponent.SetLightColor` (`self.PointLight`) (make `LinearColor` 1.0 0.0 0.0 1.0) true)
  (`LightComponent.SetIntensity` (`self.PointLight`) 10000.0)
  (`KismetSystemLibrary.Delay` 5.0)
  (`LightComponent.SetIntensity` (`self.PointLight`) 0.0))

(fn `UserConstructionScript`)