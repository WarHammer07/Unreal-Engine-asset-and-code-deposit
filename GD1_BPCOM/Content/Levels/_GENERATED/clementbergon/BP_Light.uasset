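; BP_Light is a light actor whose point light toggles on and off through a remote event on the player's character.
; On BeginPlay it casts player 0's character to BP_ThirdPersonCharacter and binds its Interrupteur event through BindEventToRemote.
; Each Interrupteur call flips IsActivated and switches the PointLight intensity between zero and a fixed bright value.
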(event `self.ReceiveBeginPlay`
  (bind _asbp_third_person_character (cast `/Game/ThirdPerson/Blueprints/BP_ThirdPersonCharacter` (`GameplayStatics.GetPlayerCharacter` 0)))
  (add `/Game/ThirdPerson/Blueprints/BP_ThirdPersonCharacter.Remote` _asbp_third_person_character (delegate `Interrupteur`)))

(event `Interrupteur`
  (bind _pointlight (`self.PointLight`))
  (if (`self.IsActivated`)
    (`LightComponent.SetIntensity` _pointlight 0.0)
    (set `self.IsActivated` false)
    (else
      (`LightComponent.SetIntensity` _pointlight 50000.0)
      (set `self.IsActivated` true))))

(fn `UserConstructionScript`)