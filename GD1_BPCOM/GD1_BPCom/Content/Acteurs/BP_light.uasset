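; BP_light is a switchable light actor that the player toggles remotely.
; On BeginPlay it casts the player character to BP_ThirdPersonCharacter and binds its Interrupteur event to that character's Telecommande event dispatcher.
; Each dispatch flips the IsActif flag and sets the PointLight intensity to either zero or full brightness.
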(event `self.ReceiveBeginPlay`
  ; On "écoute" un évènement de type "dispatch" en provenance du joueur qui s'appelle "Telecommande"
  (bind _asbp_third_person_character (cast `/Game/ThirdPerson/Blueprints/BP_ThirdPersonCharacter` (`GameplayStatics.GetPlayerCharacter` 0)))
  (add `/Game/ThirdPerson/Blueprints/BP_ThirdPersonCharacter.telecommande` _asbp_third_person_character (delegate `Interrupteur`)))

(event `Interrupteur`
  (bind _pointlight (`self.PointLight`))
  ; Le Custom Event Interrupteur est éxécuté si on "entend" l'ordre "Telecommande"
  (if (`self.isActif`)
    ;; C'est allumé, donc on doit éteindre
    (`LightComponent.SetIntensity` _pointlight 0.0)
    (set `self.isActif` false)
    (else
      ;; C'est éteint, donc faut allumer
      (`LightComponent.SetIntensity` _pointlight 50000.0)
      (set `self.isActif` true))))

(fn `UserConstructionScript`)