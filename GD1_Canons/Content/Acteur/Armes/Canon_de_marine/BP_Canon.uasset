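; BP_Canon is a naval cannon that fires BP_Boulet cannonballs and tilts in pitch.
; Tire waits a random short delay, triggers explosion particles and audio, then spawns the ball at SpawnPoint.
; Recoil uses opposing timed impulses on Canon plus a downward kick on Fut, while Monter and Descendre step Fut's pitch within limits.
; The alternate Audio2 branch never runs because RandomInteger(1) always returns zero.
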(event `Tire`
  (bind _canon (`self.Canon`))
  (bind _canon_2 (`self.Canon`))
  (`KismetSystemLibrary.Delay` (`KismetMathLibrary.RandomFloatInRange` 0.0 0.5))
  (if (== (`KismetMathLibrary.RandomInteger` 1) 0)
    (`|ExecutionSequence`
      (:`then_0`
        (`ActorComponent.Activate` (`self.P_Explosion`) true))
      (:`then_1`
        (`ActorComponent.Activate` (`self.Audio`) true)
        (`|SpawnActorFromClass` "/Game/Acteur/Armes/Boulet/BP_Boulet.BP_Boulet_C" (`SceneComponent.K2_GetComponentToWorld` (`self.SpawnPoint`)) "Undefined" "MultiplyWithRoot" null null :!label _label)
        (`PrimitiveComponent.AddImpulse` _canon_2 (* (`SceneComponent.GetForwardVector` _canon_2) (250.0 0.0 0.0)) "None" true)
        (`PrimitiveComponent.AddImpulseAtLocation` (`self.Fut`) (0.0 0.0 -500.0) (-150.0 0.0 0.0) "None")
        (`KismetSystemLibrary.Delay` 0.2)
        (`PrimitiveComponent.AddImpulse` _canon (* (`SceneComponent.GetForwardVector` _canon) (-300.0 0.0 0.0)) "None" true)))
    (else
      (`|ExecutionSequence`
        (:`then_0`
          (`ActorComponent.Activate` (`self.P_Explosion`) true))
        (:`then_1`
          (`ActorComponent.Activate` (`self.Audio2`) true)
          (goto _label))))))

(event `Monter`
  (bind (_relativerotation_roll _relativerotation_pitch) (`KismetMathLibrary.BreakRotator` (`SceneComponent.RelativeRotation` (`self.Fut`))))
  (if (> _relativerotation_pitch -15.0)
    (`SceneComponent.K2_AddLocalRotation` (`self.Fut`) (struct :`Pitch` -2.5) false false)))

(event `Descendre`
  (bind (_relativerotation_roll _relativerotation_pitch) (`KismetMathLibrary.BreakRotator` (`SceneComponent.RelativeRotation` (`self.Fut`))))
  (if (< _relativerotation_pitch 5.0)
    (`SceneComponent.K2_AddLocalRotation` (`self.Fut`) (struct :`Pitch` 2.5) false false)))

(fn `UserConstructionScript`)