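; GM_Jeu is the game mode that manages the player's health and its HUD display.
; On BeginPlay it creates the HUD_BarreVie widget, caches the third-person character and restores its HP from the GI_gameBlueprint game instance.
; MajHP adds a signed amount to the player's HP, clamps it between 0 and 100, then refreshes the HUD text and health bar.
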(event `self.ReceiveBeginPlay`
  (`|ExecutionSequence`
    (:`then_0`
      ; Création du HUD (mise en mémoire)
      (bind _returnvalue (`|CreateWidget` "/Game/HUD/HUD_BarreVie.HUD_BarreVie_C" (`GameplayStatics.GetPlayerController` 0)))
      ; Affichage à l'écran
      (bind _output_get (set `self.HUD` _returnvalue))
      (`UserWidget.AddToViewport` _output_get 0))
    (:`then_1`
      (bind _asbp_third_person_character (cast `/Game/ThirdPerson/Blueprints/BP_ThirdPersonCharacter` (`GameplayStatics.GetPlayerCharacter` 0)))
      (set `self.Joueur` _asbp_third_person_character))
    (:`then_2`
      ; Attribution des HP du Game Instance au joueur
      (bind _asgi_game_blueprint (cast `/Game/CORE/GI_gameBlueprint` (`GameplayStatics.GetGameInstance`)))
      (set `/Game/ThirdPerson/Blueprints/BP_ThirdPersonCharacter.HP` (`/Game/CORE/GI_gameBlueprint.HP` _asgi_game_blueprint) (`self.Joueur`))
      (`self.MajHP` 0))))

(event `MajHP`
  (params (HP :type Integer))
  (bind _output_get (set `/Game/ThirdPerson/Blueprints/BP_ThirdPersonCharacter.HP` (+ HP (`/Game/ThirdPerson/Blueprints/BP_ThirdPersonCharacter.HP` (`self.Joueur`))) (`self.Joueur`)))
  (`|ExecutionSequence`
    (:`then_0`
      (if (< _output_get 0)
        (set `/Game/ThirdPerson/Blueprints/BP_ThirdPersonCharacter.HP` 0 (`self.Joueur`))))
    (:`then_1`
      (if (> _output_get 100)
        (set `/Game/ThirdPerson/Blueprints/BP_ThirdPersonCharacter.HP` 100 (`self.Joueur`))))
    (:`then_2`
      (`TextBlock.SetText` (`/Game/HUD/HUD_BarreVie.AffHP` (`self.HUD`)) (`KismetTextLibrary.Conv_IntToText` _output_get)))
    (:`then_3`
      (`ProgressBar.SetPercent` (`/Game/HUD/HUD_BarreVie.BarreVie` (`self.HUD`)) (/ (`KismetMathLibrary.Conv_IntToDouble` _output_get) 100.0)))))

(fn `UserConstructionScript`)