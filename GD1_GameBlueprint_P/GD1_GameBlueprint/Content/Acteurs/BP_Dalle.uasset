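; BP_Dalle is a floor tile actor that heals or damages the player who steps on it, depending on its Type enum.
; The construction script tints the Dalle mesh green for the first type and red otherwise through the Couleur material parameter.
; When the player character overlaps the Box, it passes a positive or negative HP amount to GM_Jeu's MajHP, using a game mode reference cached at BeginPlay.
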(event `self.ReceiveBeginPlay`
  (bind _asgm_jeu (cast `/Game/CORE/GM_Jeu` (`GameplayStatics.GetGameMode`)))
  (set `self.GM Jeu` _asgm_jeu))

(event `self.Box.OnComponentBeginOverlap`
  (params (OverlappedComponent :type "PrimitiveComponent Object Reference") (OtherActor :type "Actor Object Reference") (OtherComp :type "PrimitiveComponent Object Reference") (OtherBodyIndex :type Integer) (bFromSweep :type Boolean) (SweepResult :type "HitResult Structure (by ref)"))
  (if (== OtherActor (`GameplayStatics.GetPlayerCharacter` 0))
    (if (`|EnumEquality` (`self.Type`) "NewEnumerator0")
      (`/Game/CORE/GM_Jeu.MajHP` (`self.GM Jeu`) (`self.HP`))
      (else
        (`/Game/CORE/GM_Jeu.MajHP` (`self.GM Jeu`) (* (`self.HP`) -1))))))

(fn `UserConstructionScript`
  (bind _dalle (`self.Dalle`))
  (if (`|EnumEquality` (`self.Type`) "NewEnumerator0")
    (`MeshComponent.SetVectorParameterValueOnMaterials` _dalle "Couleur" (0.0 1.0 0.0))
    (else
      (`MeshComponent.SetVectorParameterValueOnMaterials` _dalle "Couleur" (1.0 0.0 0.0)))))