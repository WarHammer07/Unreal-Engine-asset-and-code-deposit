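; BP_Teleporteur is a level-exit teleporter that moves the player to another level on contact.
; BeginPlay caches the GI_gameBlueprint game instance and the player's BP_ThirdPersonCharacter.
; When that player overlaps the Zone component, it saves their HP in the game instance so the value outlives the level change.
; It then opens the level named by the editor-selected Niveau enum, converted from string to name.
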(event `self.ReceiveBeginPlay`
  (`|ExecutionSequence`
    (:`then_0`
      (bind _asgi_game_blueprint (cast `/Game/CORE/GI_gameBlueprint` (`GameplayStatics.GetGameInstance`)))
      (set `self.Game Instance` _asgi_game_blueprint))
    (:`then_1`
      (bind _asbp_third_person_character (cast `/Game/ThirdPerson/Blueprints/BP_ThirdPersonCharacter` (`GameplayStatics.GetPlayerCharacter` 0)))
      (set `self.Joueur` _asbp_third_person_character))))

(event `self.Zone.OnComponentBeginOverlap`
  (params (OverlappedComponent :type "PrimitiveComponent Object Reference") (OtherActor :type "Actor Object Reference") (OtherComp :type "PrimitiveComponent Object Reference") (OtherBodyIndex :type Integer) (bFromSweep :type Boolean) (SweepResult :type "HitResult Structure (by ref)"))
  ; On vérifie que ce soit bien le joueur qui marche sur le téléporteur
  (if (== OtherActor (`self.Joueur`))
    ; Stockage des HP's dans l'instance
    (set `/Game/CORE/GI_gameBlueprint.HP` (`/Game/ThirdPerson/Blueprints/BP_ThirdPersonCharacter.HP` (`self.Joueur`)) (`self.Game Instance`))
    ; On change de level en précisant le nom
    (`GameplayStatics.OpenLevel` (`KismetStringLibrary.Conv_StringToName` (`|GetEnumeratorNameAsString` (`self.Niveau`))))))

(fn `UserConstructionScript`)