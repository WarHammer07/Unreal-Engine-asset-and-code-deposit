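; Door actor that slides its mesh vertically between closed and open positions.
; Ouvre plays a timeline that lerps the mesh's relative location, and Ferme reverses it.
; The construction script records the start location, derives the open position by lowering Z by Ouverture, and sets the timeline play rate from Vitesse.
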(event `Ouvre`
  (bind (_direction _variation) (`Timeline|Timeline` :!label _label)
    (:`Update`
      (`SceneComponent.K2_SetRelativeLocation` (`self.SM_porte`) (`KismetMathLibrary.VLerp` (`self.PosDep`) (`self.PosArr`) _variation) false false))))

(event `Ferme`
  (goto _label :!via `Reverse`))

(fn `UserConstructionScript`
  (locals (NewLocalVar :type "Vector Structure" :default (0.0 0.0 0.0)))
  (`|ExecutionSequence`
    (:`then_0`
      (bind _output_get (set `self.PosDep` (`SceneComponent.RelativeLocation` (`self.SM_porte`))))
      (set `self.PosArr` (`KismetMathLibrary.MakeVector` (.x _output_get) (.y _output_get) (- (.z _output_get) (`self.Ouverture`)))))
    (:`then_1`
      (`TimelineComponent.SetPlayRate` (`self.Timeline`) (`self.Vitesse`)))))