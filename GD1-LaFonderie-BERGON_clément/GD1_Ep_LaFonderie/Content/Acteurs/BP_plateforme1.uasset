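; BP_plateforme1 is a moving platform actor that slides its SMPlateforme component between a start and an end position.
; On BeginPlay a Timeline plays, and its Variation track drives a vector lerp from PosDepart to PosArrivee, applied as relative location without sweep.
; The construction script places the Previ component slightly above PosArrivee, apparently as a preview of the destination.
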(event `self.ReceiveBeginPlay`
  (bind (_direction _variation) (`Timeline|Timeline`)
    (:`Update`
      (`SceneComponent.K2_SetRelativeLocation` (`self.SM_plateforme`) (`KismetMathLibrary.VLerp` (`self.PosDepart`) (`self.PosArrivee`) _variation) false false))))

(fn `UserConstructionScript`
  (bind (_posarrivee_x _posarrivee_y _posarrivee_z) (`KismetMathLibrary.BreakVector` (`self.posArrivee`)))
  (`SceneComponent.K2_SetRelativeLocation` (`self.Previ`) (`KismetMathLibrary.MakeVector` _posarrivee_x _posarrivee_y (+ _posarrivee_z 25.0)) false false))