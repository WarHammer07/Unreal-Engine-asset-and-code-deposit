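; BP_Dalle06 is a slab actor that moves between two positions while the player is inside its collision volume.
; The Deplacement timeline starts at BeginPlay with a zero play rate and lerps the slab's relative location from PosDepart to PosArrivee.
; Player overlap toggles the play rate, so movement pauses on exit and resumes in place on entry.
; The same events make the material glow bright green on entry and dim it on exit.
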(event `self.ReceiveBeginPlay`
  ; On stoppe de suite l'animation en réglant le PlayRate de notre Timeline à zéro
  (`TimelineComponent.SetPlayRate` (`self.Deplacement`) 0.0)
  (bind (_direction _variation) (`Timeline|Deplacement`)
    (:`Update`
      (`SceneComponent.K2_SetRelativeLocation` (`self.Dalle`) (`KismetMathLibrary.VLerp` (`self.posDepart`) (`self.posArrivee`) _variation) false false))))

(event `self.Collision.OnComponentBeginOverlap`
  (params (OverlappedComponent :type "PrimitiveComponent Object Reference") (OtherActor :type "Actor Object Reference") (OtherComp :type "PrimitiveComponent Object Reference") (OtherBodyIndex :type Integer) (bFromSweep :type Boolean) (SweepResult :type "HitResult Structure (by ref)"))
  ; On check si c'est bien le joueur qui entre
  (if (== OtherActor (`GameplayStatics.GetPlayerCharacter` 0))
    ; Gestion de la Teinte
    (`MeshComponent.SetVectorParameterValueOnMaterials` (`self.Dalle`) "Teinte" (0.0 1.0 0.0))
    ; Gestion de l'Intensité
    (`MeshComponent.SetScalarParameterValueOnMaterials` (`self.Dalle`) "Intensité" 500.0)
    ; Gestion de la vitesse de lecture de l'animation
    (`TimelineComponent.SetPlayRate` (`self.Deplacement`) 1.0)))

(event `self.Collision.OnComponentEndOverlap`
  (params (OverlappedComponent :type "PrimitiveComponent Object Reference") (OtherActor :type "Actor Object Reference") (OtherComp :type "PrimitiveComponent Object Reference") (OtherBodyIndex :type Integer))
  ; On check si c'est bien le joueur qui sort
  (if (== OtherActor (`GameplayStatics.GetPlayerCharacter` 0))
    ; Gestion de la Teinte
    (`MeshComponent.SetVectorParameterValueOnMaterials` (`self.Dalle`) "Teinte" (0.0 0.1 0.0))
    ; Gestion de l'Intensité
    (`MeshComponent.SetScalarParameterValueOnMaterials` (`self.Dalle`) "Intensité" 0.0)
    ; Gestion de la vitesse de lecture de l'animation
    (`TimelineComponent.SetPlayRate` (`self.Deplacement`) 0.0)))

(fn `UserConstructionScript`)