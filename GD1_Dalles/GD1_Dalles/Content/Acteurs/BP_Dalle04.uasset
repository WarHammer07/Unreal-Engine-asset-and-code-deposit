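; BP_Dalle04 is a moving slab actor that travels between a start and an arrival position.
; On BeginPlay, the Deplacement timeline drives a lerp from PosDepart to PosArrivee, setting the slab's relative location each update without sweep.
; The construction script moves a preview volume to the arrival position, set by a 3D gizmo, with a small vertical offset to visualize the destination.
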(event `self.ReceiveBeginPlay`
  (bind (_direction _variation) (`Timeline|Deplacement`)
    (:`Update`
      (`SceneComponent.K2_SetRelativeLocation` (`self.Dalle`) (`KismetMathLibrary.VLerp` (`self.posDepart`) (`self.posArrivee`) _variation) false false))))

(fn `UserConstructionScript`
  (bind (_posarrivee_x _posarrivee_y _posarrivee_z) (`KismetMathLibrary.BreakVector` (`self.posArrivee`)))
  ; On récupère la position d'arrivée (représentée par un petit Gizmo 3D) et on déplace notre volume de prévisualisation aux mêmes coordonnées.
  (`SceneComponent.K2_SetRelativeLocation` (`self.previsualisation`) (`KismetMathLibrary.MakeVector` _posarrivee_x _posarrivee_y (+ _posarrivee_z 25.0)) false false))