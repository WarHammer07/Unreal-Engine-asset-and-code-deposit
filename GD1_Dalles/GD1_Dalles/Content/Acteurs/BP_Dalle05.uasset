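; BP_Dalle05 is a moving slab platform that travels along a spline and lights up while the player stands in its collision volume.
; The construction script caches the spline length, and a Timeline at a configurable speed maps its output to a distance along the spline, setting the slab's relative location and yaw.
; Player overlap begin and end switch material tint and intensity parameters between bright green glow and dim unlit state.
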(event `self.ReceiveBeginPlay`
  ; Modification de la vitesse de lecture de la Timeline
  (`TimelineComponent.SetPlayRate` (`self.Deplacement`) (`self.vitesse`))
  (bind (_direction _variation) (`Timeline|Deplacement`)
    (:`Update`
      (bind _returnvalue (`SplineComponent.GetTransformAtDistanceAlongSpline` (`self.Spline`) (* _variation (`self.longueurSpline`)) "Local" false))
      ; On modifie la position relative de la Dalle
      (`SceneComponent.K2_SetRelativeLocation` (`self.Dalle`) (.location _returnvalue) false false)
      ; On modifie l'orientation relative de la Dalle
      (`SceneComponent.K2_SetRelativeRotation` (`self.Dalle`) (`KismetMathLibrary.MakeRotator` 0.0 0.0 (.yaw (.rotation _returnvalue))) false false))))

(event `self.Collision.OnComponentBeginOverlap`
  (params (OverlappedComponent :type "PrimitiveComponent Object Reference") (OtherActor :type "Actor Object Reference") (OtherComp :type "PrimitiveComponent Object Reference") (OtherBodyIndex :type Integer) (bFromSweep :type Boolean) (SweepResult :type "HitResult Structure (by ref)"))
  ;[0 0.8755 1 0.3304 64] Gestion de la lumière
  ;; On check si c'est bien le joueur qui entre
  (if (== OtherActor (`GameplayStatics.GetPlayerCharacter` 0))
    ;; Gestion de la Teinte
    (`MeshComponent.SetVectorParameterValueOnMaterials` (`self.Dalle`) "Teinte" (0.0 1.0 0.0))
    ;; Gestion de l'Intensité
    (`MeshComponent.SetScalarParameterValueOnMaterials` (`self.Dalle`) "Intensité" 500.0)))

(event `self.Collision.OnComponentEndOverlap`
  (params (OverlappedComponent :type "PrimitiveComponent Object Reference") (OtherActor :type "Actor Object Reference") (OtherComp :type "PrimitiveComponent Object Reference") (OtherBodyIndex :type Integer))
  ;[0 0.8755 1 0.3304 64] Gestion de la lumière
  ;; On check si c'est bien le joueur qui sort
  (if (== OtherActor (`GameplayStatics.GetPlayerCharacter` 0))
    ;; Gestion de la Teinte
    (`MeshComponent.SetVectorParameterValueOnMaterials` (`self.Dalle`) "Teinte" (0.0 0.1 0.0))
    ;; Gestion de l'Intensité
    (`MeshComponent.SetScalarParameterValueOnMaterials` (`self.Dalle`) "Intensité" 0.0)))

(fn `UserConstructionScript`
  ; Rcupération et enregistrement de la longueur de la spline à chaque fois qu'on modifie notre blueprint dans l'éditeur
  (set `self.longueurSpline` (`SplineComponent.GetSplineLength` (`self.Spline`))))